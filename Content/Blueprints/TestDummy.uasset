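; A test dummy actor that takes damage through a health variable and destroys itself when that runs out.
; AnyDamage subtracts health, moves the static mesh to a fixed raised relative position, and blocks further damage for a short delay.
; Tick polls health and prints a death message before destroying the actor.
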(event EventBeginPlay)

(event EventTick
  (params (DeltaSeconds :type Float%20%28single-precision%29))
  (if (<= (Variables|Default|GetHaitchPee) 0.0)
    (Development|PrintString "I died!")
    (Actor|DestroyActor)))

(event Game|Damage|EventAnyDamage
  (params (Damage :type Float%20%28single-precision%29) (DamageType :type Damage%20Type%20Object%20Reference) (InstigatedBy :type Controller%20Object%20Reference) (DamageCauser :type Actor%20Object%20Reference))
  (if (Variables|Default|GetcanBeDmg)
    (Variables|Default|SetHaitchPee (- (Variables|Default|GetHaitchPee) Damage))
    (Components|MoveComponentTo (Variables|Default|GetStaticMesh) "0, 0,200.000000" "0, 0, 0" false false 0.2 false)
    (Variables|Default|SetcanBeDmg false)
    (Utilities|FlowControl|Delay 0.2)
    (Variables|Default|SetcanBeDmg true)))

(fn ConstructionScript)